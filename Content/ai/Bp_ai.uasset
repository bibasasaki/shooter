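; Zombie enemy character that registers with BP_FirstPersonGameMode on spawn, takes damage and attacks pawns in melee.
; Attack plays a montage and immediately sphere-traces a short distance forward to damage the pawn hit.
; Death plays a montage and sound, stops movement, then after a delay decrements Enemyalive, calls Enemyleft and destroys the actor.
; BeginPlay increments both Enemyalive and Amountalive, but the Amountalive decrement is unconnected and never runs.
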(event EventAttack
  (bind _returnvalue (Transformation|GetActorLocation))
  (if (not (Variables|Default|Getisdead))
    (Animation|Montage|PlayMontage (Variables|Character|GetMesh) "/Game/ai/source/attack_Montage.attack_Montage"
      (:then
        (bind (_outhit _returnvalue_2) (Collision|SphereTraceForObjects _returnvalue (+ _returnvalue (* (Math|Vector|GetForwardVector (Transformation|GetActorRotation)) 1.7e+02)) 3e+01 (Utilities|Array|MakeArray "ObjectTypeQuery3") false 0 "None"))
        (if _returnvalue_2
          (Game|Damage|ApplyDamage (.HitActor (Collision|BreakHitResult _outhit)) 1e+01 0 0))))))

(event EventBeginPlay
  (Utilities|FlowControl|Sequence
    (:then_0
      (bind _asbp_first_person_game_mode (Utilities|Casting|CastToBP_FirstPersonGameMode (Game|GetGameMode)))
      (Math|Integer|IncrementInt (Variables|/Game/FirstPerson/Blueprints/BP_FirstPersonGameMode.BP_FirstPersonGameMode_C|Getenemyalive _asbp_first_person_game_mode)))
    (:then_1
      (bind _asbp_first_person_game_mode_2 (Utilities|Casting|CastToBP_FirstPersonGameMode (Game|GetGameMode)))
      (Variables|/Game/FirstPerson/Blueprints/BP_FirstPersonGameMode.BP_FirstPersonGameMode_C|Setamountalive _asbp_first_person_game_mode_2 (+ (Variables|/Game/FirstPerson/Blueprints/BP_FirstPersonGameMode.BP_FirstPersonGameMode_C|Getamountalive _asbp_first_person_game_mode_2) 1)))))

(event Game|Damage|EventAnyDamage
  (params (Damage :type Float%20%28single-precision%29) (DamageType :type Damage%20Type%20Object%20Reference) (InstigatedBy :type Controller%20Object%20Reference) (DamageCauser :type Actor%20Object%20Reference))
  (Variables|Default|Sethealth (- (Variables|Default|Gethealth) Damage))
  (if (<= (Variables|Default|Gethealth) 0.0)
    (if (not (Variables|Default|Getisdead))
      (Variables|Default|Setisdead true)
      (Animation|Montage|PlayMontage (Variables|Character|GetMesh) "/Game/ai/source/death_Montage.death_Montage"
        (:then
          (Pawn|Components|CharacterMovement|DisableMovement (Variables|Character|GetCharacterMovement))
          (Audio|PlaySoundatLocation "/Game/FirstPerson/music/zombie_3.zombie_3" (Transformation|GetActorLocation) "0, 0, 0" 1.0 1.0 0.0 0 0 0 0)
          (Utilities|FlowControl|Delay 5.0)
          (bind _asbp_first_person_game_mode (Utilities|Casting|CastToBP_FirstPersonGameMode (Game|GetGameMode)))
          (Math|Integer|DecrementInt (Variables|/Game/FirstPerson/Blueprints/BP_FirstPersonGameMode.BP_FirstPersonGameMode_C|Getenemyalive _asbp_first_person_game_mode)
            (:%20%20
              (Default|Enemyleft _asbp_first_person_game_mode)
              (Actor|DestroyActor))))))))

(fn ConstructionScript)